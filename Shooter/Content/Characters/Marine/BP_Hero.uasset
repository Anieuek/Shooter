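; BP_Hero is the player-controlled Marine character, with world-axis movement, mouse-driven facing and a firing effect.
; Each tick, when mouse velocity exceeds a dead zone, control rotation interpolates toward the yaw of the mouse's movement direction, rather than toward a cursor position.
; Pressing fire activates a particle system and shooting sound; releasing stops both and plays an end sound, with no projectile or damage logic here.
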(event `InputAction|WeaponFired`
  (params (Key :type "Key Structure"))
  ;[1 0.0176 0] Shooting
  (:`Pressed`
    (`self.StartFired`))
  (:`Released`
    (`self.StopFired`)))

(event `InputAxis|MoveForwardBackward`
  (params (AxisValue :type "Float (single-precision)"))
  ;[1 1 1] Movment
  (`self.AddMovementInput` (0.0 1.0 0.0) AxisValue))

(event `InputAxis|MoveRightLeft`
  (params (AxisValue :type "Float (single-precision)"))
  ;[1 1 1] Movment
  (`self.AddMovementInput` (1.0 0.0 0.0) AxisValue))

(event `self.ReceiveTick`
  (params (DeltaSeconds :type "Float (single-precision)"))
  ;[0.06542 0.009607 1] Rotation
  (`self.UpdatePlayerRotation`))

(fn `getMouseVelocity`
  (returns (ReturnValue :type "Vector2D Structure"))
  (bind (_deltax _deltay) (`PlayerController.GetInputMouseDelta` (`GameplayStatics.GetPlayerController` 0)))
  ;[1 1 1] ustala jak szybko myszka machamy
  (return (/ (`KismetMathLibrary.MakeVector2D` _deltax _deltay) (`GameplayStatics.GetWorldDeltaSeconds`))))

(fn `IsMouseAboveDeadZone`
  (returns (ReturnValue :type Boolean))
  (return (> (`KismetMathLibrary.VSize2D` (`self.getMouseVelocity`)) (`self.MouseDeadZone`))))

(fn `StartFired`
  (`ActorComponent.Activate` (`self.ParticleSystem`) false)
  (bind _returnvalue (`GameplayStatics.SpawnSound2D` "/Game/Sounds/Weapon_AssaultRifle/Stereo/SC_Shoot.SC_Shoot" 1.0 1.0 0.0 null))
  (set `self.SCWeaponSound` _returnvalue))

(fn `StopFired`
  (`ActorComponent.Deactivate` (`self.ParticleSystem`))
  (`AudioComponent.Stop` (`self.SCWeaponSound`))
  (bind _returnvalue (`GameplayStatics.SpawnSound2D` "/Game/Sounds/Weapon_AssaultRifle/Stereo/SC_ShootEnd.SC_ShootEnd" 1.0 1.0 0.0 null))
  (set `self.SCWeaponShootEnd` _returnvalue))

(fn `UpdatePlayerRotation`
  (bind _returnvalue (`GameplayStatics.GetPlayerController` 0))
  (bind (_returnvalue_x _returnvalue_y) (`KismetMathLibrary.BreakVector2D` (`self.getMouseVelocity`)))
  (if (`self.IsMouseAboveDeadZone`)
    (`Controller.SetControlRotation` _returnvalue (`KismetMathLibrary.RInterpTo` (`Controller.GetControlRotation` _returnvalue) (`KismetMathLibrary.MakeRotator` 0.0 0.0 (`KismetMathLibrary.DegAtan2` _returnvalue_x _returnvalue_y)) (`GameplayStatics.GetWorldDeltaSeconds`) (`self.DeltaTimeMultiplier`)))))

(fn `UserConstructionScript`)